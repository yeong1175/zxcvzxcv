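; Enemy character Blueprint that takes damage, reacts to hits, dies and acquires the player as a target.
; Damage feeds the stat component, whose death result flags the anim Blueprint, disables capsule collision and destroys the actor after a delay.
; Non-lethal hits play a randomly indexed hit montage, with the range taken from a separate TargetArray input.
; A TempDetector overlap passes the player character to the AI controller.
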(event `self.ReceiveBeginPlay`
  (bind _asabp_enemy (cast `/Game/CustomContents/Enemy/ABP_Enemy` (`SkeletalMeshComponent.GetAnimInstance` (`self.Mesh`))))
  (set `self.AnimationBp` _asabp_enemy))

(event `self.ReceiveAnyDamage`
  (params (Damage :type "Float (single-precision)") (DamageType :type "DamageType Object Reference") (InstigatedBy :type "Controller Object Reference") (DamageCauser :type "Actor Object Reference"))
  (bind _isdead (`/Game/CustomContents/ComPonents/Bpc_StatSystem.decreaseHealth` (`self.Bpc_StatSystem`) Damage))
  (bind _output_get (set `self.Is Dead` _isdead))
  (if _output_get
    (`/Game/CustomContents/Enemy/ABP_Enemy.SetEnemyisDead` (`self.AnimationBp`))
    (`PrimitiveComponent.SetCollisionEnabled` (`self.CapsuleComponent`) "NoCollision")
    (`KismetSystemLibrary.Delay` 10.0)
    (`self.K2_DestroyActor`)
    (else
      (`self.PlayhitAnim` (`self.HitMontague`)))))

(event `self.TempDetector.OnComponentBeginOverlap`
  (params (OverlappedComponent :type "PrimitiveComponent Object Reference") (OtherActor :type "Actor Object Reference") (OtherComp :type "PrimitiveComponent Object Reference") (OtherBodyIndex :type Integer) (bFromSweep :type Boolean) (SweepResult :type "HitResult Structure (by ref)"))
  (bind _asbp_player_character (cast `/Game/CustomContents/Player/Bp_PlayerCharacter` OtherActor))
  (bind _asaic_enemy (cast `/Game/CustomContents/Enemy/AIC_Enemy` (`AIBlueprintHelperLibrary.GetAIController` self)))
  (`/Game/CustomContents/Enemy/AIC_Enemy.SetTarget` _asaic_enemy _asbp_player_character))

(fn `PlayhitAnim`
  (params (Array :type "Array of AnimMontage Object Reference") (TargetArray :type "Array of AnimMontage Object Reference (by ref)"))
  (`self.PlayAnimMontage` (`|GetArrayItem` Array (`KismetMathLibrary.RandomIntegerInRange` 0 (- (`KismetArrayLibrary.Array_Length` TargetArray) 1)))))

(fn `UserConstructionScript`)