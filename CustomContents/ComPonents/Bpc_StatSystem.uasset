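; Bpc_StatSystem is a component that tracks health and death state, set to maximum health on BeginPlay.
; DecreaseHealth subtracts damage, prints the remaining health or a death message, and below zero clamps to zero and sets and returns IsDead.
; IncreaseHealth is unfinished: it sets health to zero before the maximum clamp, leaving the addition of HealthPoint unconnected.
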(event `self.ReceiveBeginPlay`
  (`self.initializestat`))

(fn `decreaseHealth`
  (params (DamagePoint :type "Float (double-precision)"))
  (returns (IsDead :type Boolean))
  (set `self.Currenthealth` (- (`self.Currenthealth`) DamagePoint))
  (if (< (`self.Currenthealth`) 0.0)
    (`KismetSystemLibrary.PrintString` "death")
    (else
      (`KismetSystemLibrary.PrintString` (`KismetStringLibrary.Conv_DoubleToString` (`self.Currenthealth`)))))
  (if (< (`self.Currenthealth`) 0.0)
    (set `self.Currenthealth` 0.0)
    (bind _output_get (set `self.IsDead` true))
    (return _output_get)))

(fn `IncreaseHealth`
  (params (HealthPoint :type "Float (double-precision)"))
  (set `self.Currenthealth` 0.0)
  (if (> (`self.Currenthealth`) (`self.Maxhealth`))
    (set `self.Currenthealth` (`self.Maxhealth`))))

(fn `initializestat`
  (set `self.Currenthealth` (`self.Maxhealth`)))