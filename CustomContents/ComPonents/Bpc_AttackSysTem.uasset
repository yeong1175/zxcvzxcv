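; Player character component that runs a four-punch melee combo (jab, straight, two hooks) from the attack input.
; Each montage's notify advances the combo counter and unlocks the next attack.
; StartAttackTrace and StopAttackTrace control a timer for a debug-drawn sphere trace from the left or right hand, picked by the counter.
; Damage is applied to the trace's hit actor without checking the hit result.
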(event `self.ReceiveBeginPlay`
  (bind _asbp_player_character (cast `/Game/CustomContents/Player/Bp_PlayerCharacter` (`self.GetOwner`)))
  (bind _output_get (set `self.PlayerCharacter` _asbp_player_character))
  (set `self.CharacterMesh` (`Character.Mesh` _output_get)))

(event `EnhancedInput|/Game/CustomContents/Player/Input/IA_Attack`
  (params (ActionValue :type Boolean) (ElapsedSeconds :type "Float (double-precision)") (TriggeredSeconds :type "Float (double-precision)") (InputAction :type "InputAction Object Reference" :default "/Game/CustomContents/Player/Input/IA_Attack.IA_Attack"))
  (bind _charactermesh (`self.CharacterMesh`))
  (:`Started`
    (if (not (`self.IsAttacking`))
      (set `self.IsAttacking` true)
      (switch `int` (`self.ComboCounter`)
        (:`0`
          (`|PlayMontage` _charactermesh "/Game/CustomContents/Animation/Montague/Attack1_Jab_Montage.Attack1_Jab_Montage"
            (:`then`
              (`KismetSystemLibrary.K2_SetTimerDelegate` :`Time` 1.0 :!label _label))
            (:`OnNotifyBegin`
              (set `self.IsAttacking` false)
              (set `self.ComboCounter` 1))))
        (:`1`
          (`|PlayMontage` _charactermesh "/Game/CustomContents/Animation/Montague/Attack2_Straight_Montage.Attack2_Straight_Montage"
            (:`then`
              (goto _label))
            (:`OnNotifyBegin`
              (set `self.IsAttacking` false)
              (set `self.ComboCounter` 2))))
        (:`2`
          (`|PlayMontage` _charactermesh "/Game/CustomContents/Animation/Montague/Attack3_Hook_Montage.Attack3_Hook_Montage"
            (:`then`
              (goto _label))
            (:`OnNotifyBegin`
              (set `self.IsAttacking` false)
              (set `self.ComboCounter` 3))))
        (:`3`
          (`|PlayMontage` _charactermesh "/Game/CustomContents/Animation/Montague/Attack4_Hook_Montage.Attack4_Hook_Montage"
            (:`then`
              (goto _label))
            (:`OnNotifyBegin`
              (set `self.IsAttacking` false)
              (set `self.ComboCounter` 0))))))))

(event `Resetcounter`
  (set `self.ComboCounter` 0))

(event `StartAttackTrace`
  (bind _returnvalue (`KismetSystemLibrary.K2_SetTimerDelegate` (delegate `AttackTrace`) 0.01))
  (set `self.AttackTimerHandler` _returnvalue))

(event `AttackTrace`
  (bind (_start _end) (`self.GetHandLocation` (`/Game/CustomContents/Player/Bp_PlayerCharacter.Lefthand` (`self.PlayerCharacter`))))
  (bind (_start_2 _end_2) (`self.GetHandLocation` (`/Game/CustomContents/Player/Bp_PlayerCharacter.Righthand` (`self.PlayerCharacter`))))
  (switch `int` (`self.ComboCounter`)
    (:`0`
      (`self.NewFunction` (`self.Base Damage`) (`self.PlayerCharacter`) _start _end :!label _label_2))
    (:`1`
      (`self.NewFunction` (`self.Base Damage`) (`self.PlayerCharacter`) _start_2 _end_2 :!label _label_3))
    (:`2`
      (goto _label_2))
    (:`3`
      (goto _label_3))))

(event `StopAttackTrace`
  (`KismetSystemLibrary.K2_ClearAndInvalidateTimerHandle` (`self.AttackTimerHandler`)))

(fn `GetHandLocation`
  (params (Hand :type "SceneComponent Object Reference"))
  (returns (Start :type "Vector Structure") (End :type "Vector Structure"))
  (return (`SceneComponent.K2_GetComponentLocation` Hand) (`KismetMathLibrary.TransformLocation` (`SceneComponent.K2_GetComponentToWorld` Hand) (+ (`SceneComponent.RelativeLocation` Hand) (20.0 0.0 0.0)))))

(fn `NewFunction`
  (params (BaseDamage :type "Float (single-precision)") (DamageCauser :type "Actor Object Reference") (Start :type "Vector Structure") (End :type "Vector Structure"))
  (bind _outhit (`KismetSystemLibrary.SphereTraceSingle` :`Start` Start :`End` End :`Radius` 20.0 :`TraceChannel` "TraceTypeQuery1" :`DrawDebugType` "ForDuration" :`DrawTime` 7.0))
  (if true
    (`GameplayStatics.ApplyDamage` (`.HitActor` (`GameplayStatics.BreakHitResult` _outhit)) BaseDamage null DamageCauser)))